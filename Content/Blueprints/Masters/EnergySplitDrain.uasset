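; EnergySplitDrain is an energy source actor with two drain behaviors, chosen by the overlapping ThirdPersonCharacter's energy level.
; On overlap, if its EnergyComponent holds energy, a level above DestructPoint triggers a drain through EnergyDestroy and destroys the actor.
; Otherwise EnergyComponent drains repeatedly on a short task delay, rechecking the threshold each pass until the character leaves.
; The remaining-energy check runs only when overlap begins.
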(event `self.ReceiveActorBeginOverlap`
  (params (OtherActor :type "Actor Object Reference"))
  ;[1 1 1] Don't even try if there isn't any energy.
  (if (> (`/Game/Blueprints/Parts/EnergyComponent.Energy` (`self.EnergyComponent`)) 0.0)
    (bind _asthird_person_character (cast `/Game/ThirdPersonBP/Blueprints/ThirdPersonCharacter` OtherActor))
    (if (> (`/Game/ThirdPersonBP/Blueprints/ThirdPersonCharacter.EnergyLevel` _asthird_person_character) (`self.Destruct Point`)) :!label _label
      (`/Game/Blueprints/Parts/EnergyComponent.DrainEnergy` (`self.EnergyDestroy`) _asthird_person_character self)
      (`self.K2_DestroyActor`)
      (else
        ;[1 1 1] Loop block
        (`/Game/Blueprints/Parts/EnergyComponent.DrainEnergy` (`self.EnergyComponent`) _asthird_person_character self)
        (`GameplayTask_WaitDelay.TaskWaitDelay` (`self.GameplayTasks`) 0.1
          (:`OnFinish`
            ;[1 1 1] Stop if player leaves area
            (if (`self.IsOverlappingActor` _asthird_person_character)
              (goto _label))))))))

(fn `UserConstructionScript`)