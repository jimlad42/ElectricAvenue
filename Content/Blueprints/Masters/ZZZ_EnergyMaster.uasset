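; Master Blueprint for an energy source that a player drains to gain energy at the cost of taking damage.
; EnergyDrain requires the player's energy to be at least a minimum and the source to hold enough for one transfer.
; On success it moves energy to the player, applies energy-source damage, spawns optional particle and sound effects at an offset, and returns true; otherwise it returns false.
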(fn `EnergyDrain`
  (params (Player :type "/Game/ThirdPersonBP/Blueprints/ThirdPersonCharacter Object Reference"))
  (returns (Success :type Boolean))
  (locals (PlayerCharacter :type "/Game/ThirdPersonBP/Blueprints/ThirdPersonCharacter Object Reference"))
  (bind _sound (`self.Sound`))
  (bind _energyrate (`self.EnergyRate`))
  (bind _particletype (`self.ParticleType`))
  (bind _returnvalue (+ (`self.K2_GetActorLocation`) (`self.Offset`)))
  (bind _energylevel (`/Game/ThirdPersonBP/Blueprints/ThirdPersonCharacter.EnergyLevel` (`local.PlayerCharacter`)))
  (set `local.PlayerCharacter` Player)
  ;[1 1 1] Does the player have enough energy?
  (if (>= _energylevel (`self.MinEnergy`))
    ;[1 1 1] Is there enough energy in the system?
    (if (>= (`self.Energy`) (`self.EnergyRate`))
      ;[1 1 1] Add and remove energy
      (set `self.Energy` (- (`self.Energy`) _energyrate))
      (set `/Game/ThirdPersonBP/Blueprints/ThirdPersonCharacter.EnergyLevel` (+ _energyrate _energylevel) (`local.PlayerCharacter`))
      ;[1 1 1] Damage the Player
      (`GameplayStatics.ApplyDamage` (`local.PlayerCharacter`) (`self.Damage`) null null "/Game/Blueprints/Masters/DamageTypeEnergySource.DamageTypeEnergySource_C")
      (`|ExecutionSequence`
        (:`then_0`
          ;[1 1 1] Play a particle there
          (`/Engine/EditorBlueprintResources/StandardMacros.IsValid` _particletype
            (:`Is Valid`
              (`GameplayStatics.SpawnEmitterAtLocation` _particletype _returnvalue))))
        (:`then_1`
          ;[1 1 1] Play a sound there
          (`/Engine/EditorBlueprintResources/StandardMacros.IsValid` _sound
            (:`Is Valid`
              (`GameplayStatics.PlaySoundAtLocation` _sound _returnvalue (struct) 1.0 1.0 0.0 null null null))))
        (:`then_2`
          (return true)))
      (else
        (return false)))
    (else
      (return false))))

(fn `UserConstructionScript`)