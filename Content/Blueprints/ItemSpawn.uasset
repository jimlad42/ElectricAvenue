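; ItemSpawn is a spawner actor that creates one SpawnItem at BeginPlay from its SpawnPoints transforms.
; Location is offset from the actor's position, while rotation and scale are used as stored.
; Location, rotation and scale each take a separate random index, so they can come from different points.
; The construction script previews every point with a colored arrow component, passing its transform through FixRotation.
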(event `self.ReceiveBeginPlay`
  (`self.SpawnItems`))

(fn `SpawnItems`
  (bind _spawn_points (`self.Spawn Points`))
  (`|SpawnActorFromClass` (`self.Spawn Item`) (`KismetMathLibrary.MakeTransform` (+ (`self.K2_GetActorLocation`) (.location (`|GetArrayItem` _spawn_points (`KismetMathLibrary.RandomIntegerInRange` 0 (`KismetArrayLibrary.Array_LastIndex` _spawn_points))))) (.rotation (`|GetArrayItem` _spawn_points (`KismetMathLibrary.RandomIntegerInRange` 0 (`KismetArrayLibrary.Array_LastIndex` _spawn_points)))) (.scale (`|GetArrayItem` _spawn_points (`KismetMathLibrary.RandomIntegerInRange` 0 (`KismetArrayLibrary.Array_LastIndex` _spawn_points))))) "Undefined" "OverrideRootScale" null null))

(fn `UserConstructionScript`
  ;[1 1 1] Editor Renders for ease.
  (for _array_element (`self.Spawn Points`)
    (bind _returnvalue (`AddComponent|NODE_AddArrowComponent-0` :`RelativeTransform` (`KismetMathLibrary.MakeTransform` (.location _array_element) (`KismetMathLibrary.ComposeRotators` (.rotation _array_element) (struct :`Yaw` 90.0)) (.scale _array_element))))
    (set `ArrowComponent.ArrowColor` (`self.ArrowColor`) _returnvalue)))