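; Test actor that acts as an energy source, draining energy to a ThirdPersonCharacter that overlaps it.
; On begin overlap it checks once that its EnergyComponent has energy, then calls DrainEnergy with the character and itself.
; A WaitDelay gameplay task repeats the drain every tenth of a second until the character leaves the area.
; The loop does not recheck remaining energy.
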(event `self.ReceiveActorBeginOverlap`
  (params (OtherActor :type "Actor Object Reference"))
  ;[1 1 1] Don't even try if there isn't any energy.
  (if (> (`/Game/Blueprints/EnergyComponent.Energy` (`self.EnergyComponent`)) 0.0)
    (bind _asthird_person_character (cast `/Game/ThirdPersonBP/Blueprints/ThirdPersonCharacter` OtherActor))
    ;[1 1 1] Loop block
    (`/Game/Blueprints/EnergyComponent.DrainEnergy` (`self.EnergyComponent`) _asthird_person_character self :!label _label)
    (`GameplayTask_WaitDelay.TaskWaitDelay` (`self.GameplayTasks`) 0.1
      (:`OnFinish`
        ;[1 1 1] Stop if player leaves area
        (if (`self.IsOverlappingActor` _asthird_person_character)
          (goto _label))))))

(fn `UserConstructionScript`)